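; AI controller for guards that runs BT_Guard on possession and detects the player through AI Perception.
; A sensed player is ignored while hidden, unless already flagged as detected.
; Otherwise it marks them detected and writes line of sight and target to the Blackboard.
; The first unhidden detection also pulses an Alerted key briefly, and lost perception never clears the line-of-sight key here.
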(event `self.ReceivePossess`
  (params (PossessedPawn :type "Pawn Object Reference"))
  (`self.RunBehaviorTree` "/Game/Characters/Guard/AI/BT_Guard.BT_Guard"))

(event `self.AIPerception.OnTargetPerceptionUpdated`
  (params (Actor :type "Actor Object Reference") (Stimulus :type "AIStimulus Structure"))
  (bind _blackboard (`self.Blackboard`))
  (bind _blackboard_2 (`self.Blackboard`))
  ;[1 1 1] First check if we sense the player
  (if (and (`self.ActorHasTag` Actor "Player") (`.bSuccessfullySensed` (break `AIStimulus` Stimulus)))
    (bind _asthird_person_character (cast `/Game/Characters/PlayerCharacter/ThirdPersonCharacter` Actor))
    ;[1 1 1] Check if they are hidden
    (if (`/Game/Characters/PlayerCharacter/ThirdPersonCharacter.IsHidden?` _asthird_person_character)
      (if (`/Game/Characters/PlayerCharacter/ThirdPersonCharacter.IsDetected?` _asthird_person_character)
        (`BlackboardComponent.SetValueAsBool` _blackboard (`self.HasLineOfSight?`) true)
        (`BlackboardComponent.SetValueAsObject` _blackboard (`self.OtherActor`) Actor)
        (`KismetSystemLibrary.PrintString` "Player Cannot Hide")
        (else
          (`KismetSystemLibrary.PrintString` "Player Hidden ")))
      (else
        ;[1 1 1] Player has been detected
        (set `/Game/Characters/PlayerCharacter/ThirdPersonCharacter.IsDetected?` true _asthird_person_character)
        (`SceneComponent.SetVisibility` (`/Game/Characters/PlayerCharacter/ThirdPersonCharacter.DetectedDebug` _asthird_person_character) true false)
        (`BlackboardComponent.SetValueAsBool` _blackboard_2 (`self.HasLineOfSight?`) true)
        (`BlackboardComponent.SetValueAsObject` _blackboard_2 (`self.OtherActor`) Actor)
        (`/Engine/EditorBlueprintResources/StandardMacros.DoOnce` false
          (:`Completed`
            (`BlackboardComponent.SetValueAsBool` _blackboard_2 (`self.Alerted?`) true)
            (`KismetSystemLibrary.Delay` 2.0)
            (`BlackboardComponent.SetValueAsBool` _blackboard_2 (`self.Alerted?`) false)))))))

(fn `UserConstructionScript`)