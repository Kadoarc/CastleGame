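; HiddenArea is a trigger volume that lets the third-person player character hide inside it.
; On overlap begin it sets the character's IsHidden flag and shows its HiddenDebug component, but only if the character is not already detected.
; On overlap end it always clears the flag and hides the debug indicator.
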(event `self.ReceiveActorBeginOverlap`
  (params (OtherActor :type "Actor Object Reference"))
  (bind _asthird_person_character (cast `/Game/ThirdPersonCPP/Blueprints/ThirdPersonCharacter` OtherActor))
  (if (not (`/Game/ThirdPersonCPP/Blueprints/ThirdPersonCharacter.IsDetected?` _asthird_person_character))
    (set `/Game/ThirdPersonCPP/Blueprints/ThirdPersonCharacter.IsHidden?` true _asthird_person_character)
    (`SceneComponent.SetVisibility` (`/Game/ThirdPersonCPP/Blueprints/ThirdPersonCharacter.HiddenDebug` _asthird_person_character) true false)))

(event `self.ReceiveActorEndOverlap`
  (params (OtherActor :type "Actor Object Reference"))
  (bind _asthird_person_character (cast `/Game/ThirdPersonCPP/Blueprints/ThirdPersonCharacter` OtherActor))
  (set `/Game/ThirdPersonCPP/Blueprints/ThirdPersonCharacter.IsHidden?` false _asthird_person_character)
  (`SceneComponent.SetVisibility` (`/Game/ThirdPersonCPP/Blueprints/ThirdPersonCharacter.HiddenDebug` _asthird_person_character) false false))

(fn `UserConstructionScript`)