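; Interactable painting that detects when the ThirdPersonCharacter is close enough to interact with it.
; Box overlap begin and end show or hide InteractText and set the character's CanInteractPainting1 flag.
; While the text is visible, Tick rotates it to face that character's follow camera.
; The interaction itself is not handled here.
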(event `self.Box.OnComponentBeginOverlap`
  (params (OverlappedComponent :type "PrimitiveComponent Object Reference") (OtherActor :type "Actor Object Reference") (OtherComp :type "PrimitiveComponent Object Reference") (OtherBodyIndex :type Integer) (bFromSweep :type Boolean) (SweepResult :type "HitResult Structure (by ref)"))
  (bind _asthird_person_character (cast `/Game/ThirdPersonCPP/Blueprints/ThirdPersonCharacter` OtherActor))
  (`SceneComponent.SetVisibility` (`self.InteractText`) true false)
  (set `/Game/ThirdPersonCPP/Blueprints/ThirdPersonCharacter.CanInteractPainting1` true _asthird_person_character))

(event `self.Box.OnComponentEndOverlap`
  (params (OverlappedComponent :type "PrimitiveComponent Object Reference") (OtherActor :type "Actor Object Reference") (OtherComp :type "PrimitiveComponent Object Reference") (OtherBodyIndex :type Integer))
  (bind _asthird_person_character (cast `/Game/ThirdPersonCPP/Blueprints/ThirdPersonCharacter` OtherActor))
  (`SceneComponent.SetVisibility` (`self.InteractText`) false false)
  (set `/Game/ThirdPersonCPP/Blueprints/ThirdPersonCharacter.CanInteractPainting1` false _asthird_person_character))

(event `self.ReceiveTick`
  (params (DeltaSeconds :type "Float (single-precision)"))
  (if (`SceneComponent.IsVisible` (`self.InteractText`))
    (bind (_returnvalue_roll _returnvalue_pitch _returnvalue_yaw) (`KismetMathLibrary.BreakRotator` (`SceneComponent.K2_GetComponentRotation` (`CastleGameCharacter.FollowCamera` (stale `self.Box.OnComponentBeginOverlap` _asthird_person_character)))))
    (bind _result (`/Engine/EditorBlueprintResources/StandardMacros.NegateFloat` _returnvalue_pitch)
      (:`  `
        (`SceneComponent.K2_SetWorldRotation` (`self.InteractText`) (`KismetMathLibrary.MakeRotator` _returnvalue_roll _result (- _returnvalue_yaw 180.0)) false false)))))

(fn `UserConstructionScript`)