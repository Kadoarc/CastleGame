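; BP_GuardCharacter is an AI guard character that supplies patrol locations along a numbered path and controls its own walk speed.
; On BeginPlay it gathers Target Points tagged "PatrolPath" plus its path number, unsorted, and applies its patrol speed.
; GetNextPatrolPoint steps an index through that array, flipping direction at either end for a back-and-forth route, and returns a location.
; The Blueprint itself issues no movement orders.
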(event `self.ReceiveBeginPlay`
  (`self.GetPatrolPath` (`self.PatrolPathNumber`))
  (`self.Update Walk Speed` (`self.PatrolSpeed`)))

(fn `GetNextPatrolPoint`
  (returns (NextPatrolLocation :type "Vector Structure"))
  ;[1 1 1] First check if we are reversing order
  (if (`self.ReversingPatrol?`)
    ;[1 1 1] Are we at the FIRST patrol point?
    (if (== (`self.CurrentPatrolIndex`) 0)
      (set `self.ReversingPatrol?` false)
      (bind _result (`/Engine/EditorBlueprintResources/StandardMacros.IncrementInt` (`self.CurrentPatrolIndex`))
        (:`  `
          (return (`self.K2_GetActorLocation` (`|GetArrayItem` (`self.PatrolPoints`) _result)))))
      (else
        (bind _result_2 (`/Engine/EditorBlueprintResources/StandardMacros.DecrementInt` (`self.CurrentPatrolIndex`))
          (:`  `
            (return (`self.K2_GetActorLocation` (`|GetArrayItem` (`self.PatrolPoints`) _result_2)))))))
    (else
      ;[1 1 1] Are we at the LAST patrol point?
      (if (== (`self.CurrentPatrolIndex`) (`self.TotalPatrolPoints`))
        (set `self.ReversingPatrol?` true)
        (bind _result_3 (`/Engine/EditorBlueprintResources/StandardMacros.DecrementInt` (`self.CurrentPatrolIndex`))
          (:`  `
            (return (`self.K2_GetActorLocation` (`|GetArrayItem` (`self.PatrolPoints`) _result_3)))))
        (else
          (bind _result_4 (`/Engine/EditorBlueprintResources/StandardMacros.IncrementInt` (`self.CurrentPatrolIndex`))
            (:`  `
              (return (`self.K2_GetActorLocation` (`|GetArrayItem` (`self.PatrolPoints`) _result_4))))))))))

(fn `GetPatrolPath`
  (params (PatrolPathNumber :type Integer))
  ;[1 1 1] Get all the Target Point actors with the corect player tag path and set it to PatrolPoints
  (bind _outactors (`GameplayStatics.GetAllActorsOfClassWithTag` "/Script/Engine.TargetPoint" (`KismetStringLibrary.Conv_StringToName` (`KismetStringLibrary.Concat_StrStr` "PatrolPath" (`KismetStringLibrary.Conv_IntToString` PatrolPathNumber)))))
  (bind _output_get (set `self.PatrolPoints` _outactors))
  (set `self.TotalPatrolPoints` (`KismetArrayLibrary.Array_LastIndex` _output_get))
  (set `self.CurrentPatrolIndex` 0))

(fn `Update Walk Speed`
  (params (`New Walk Speed` :type "Float (double-precision)"))
  (set `CharacterMovementComponent.MaxWalkSpeed` `New Walk Speed` (`self.CharacterMovement`)))

(fn `UserConstructionScript`)